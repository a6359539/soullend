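; World pickup actor for an inventory item, taking its mesh, scale and interaction radius from the item class defaults.
; Sphere overlap maintains the character's nearby-pickup list to show one name label, or picks up immediately when a pickup command is pending.
; Cursor hover swaps material and cursor.
; Pickup runs client-side, adding plain or enhanced items to the local controller's inventory, then requesting destruction through the character's server call.
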(event OnComponentBeginOverlap(Sphere)
  (params (OverlappedComponent :type Primitive%20Component%20Object%20Reference) (OtherActor :type Actor%20Object%20Reference) (OtherComp :type Primitive%20Component%20Object%20Reference) (OtherBodyIndex :type Integer) (bFromSweep :type Boolean) (SweepResult :type Hit%20Result%20Structure%20%28by%20ref%29))
  (bind _asbasic_character (Utilities|Casting|CastToBasicCharacter OtherActor))
  (if (Variables|Default|GetHasPickupCommand?)
    (CallFunction|OnPickedUp _asbasic_character)
    (elif (> (Utilities|Array|Length (Variables|/Game/RPG/BasicCharacter/BasicCharacter.BasicCharacter_C|GetNearbyPickupActors _asbasic_character)) 0)
      (Utilities|Array|Add (Variables|/Game/RPG/BasicCharacter/BasicCharacter.BasicCharacter_C|GetNearbyPickupActors _asbasic_character) self)
      (else
        (Rendering|SetVisibility (Variables|Default|GetPickupText) true false)
        (Utilities|Array|Add (Variables|/Game/RPG/BasicCharacter/BasicCharacter.BasicCharacter_C|GetNearbyPickupActors _asbasic_character) self)
        (Variables|Default|SetIsInRange? true)))))

(event OnEndCursorOver(StaticMesh)
  (params (TouchedComponent :type Primitive%20Component%20Object%20Reference))
  (CallFunction|OnUnHovered))

(event OnComponentEndOverlap(Sphere)
  (params (OverlappedComponent :type Primitive%20Component%20Object%20Reference) (OtherActor :type Actor%20Object%20Reference) (OtherComp :type Primitive%20Component%20Object%20Reference) (OtherBodyIndex :type Integer))
  (bind _asbasic_character (Utilities|Casting|CastToBasicCharacter OtherActor))
  (Variables|Default|SetIsInRange? false)
  (if (and (Utilities|IsValid (Utilities|Array|Get(acopy) (Variables|/Game/RPG/BasicCharacter/BasicCharacter.BasicCharacter_C|GetNearbyPickupActors _asbasic_character))) (== (Utilities|Array|Get(acopy) (Variables|/Game/RPG/BasicCharacter/BasicCharacter.BasicCharacter_C|GetNearbyPickupActors _asbasic_character)) self))
    (Rendering|SetVisibility (Variables|Default|GetPickupText) false false)
    (Utilities|Array|RemoveItem (Variables|/Game/RPG/BasicCharacter/BasicCharacter.BasicCharacter_C|GetNearbyPickupActors _asbasic_character) self)
    (Utilities|IsValid (Utilities|Array|Get(acopy) (Variables|/Game/RPG/BasicCharacter/BasicCharacter.BasicCharacter_C|GetNearbyPickupActors _asbasic_character))
      (:Is%20Valid
        (Rendering|SetVisibility (Variables|BP_PickUpActor_C|GetPickupText (Utilities|Array|Get(acopy) (Variables|/Game/RPG/BasicCharacter/BasicCharacter.BasicCharacter_C|GetNearbyPickupActors _asbasic_character))) true false)))
    (else
      (Utilities|Array|RemoveItem (Variables|/Game/RPG/BasicCharacter/BasicCharacter.BasicCharacter_C|GetNearbyPickupActors _asbasic_character) self))))

(event OnBeginCursorOver(StaticMesh)
  (params (TouchedComponent :type Primitive%20Component%20Object%20Reference))
  (CallFunction|OnHovered)
  (Development|PrintString "???"))

(event Custom|C2S_DestroyActor
  (Actor|DestroyActor))

(event Custom|OnPickedUp
  (params (BaiscChar :type Basic%20Character%20Object%20Reference))
  (bind _returnvalue (Game|GetPlayerController 0))
  (bind _nearbypickupactors (Variables|/Game/RPG/BasicCharacter/BasicCharacter.BasicCharacter_C|GetNearbyPickupActors BaiscChar))
  (bind _itemtoadd (Variables|Default|GetItemToAdd))
  (bind _asbpc_maincontroller (Utilities|Casting|CastToBPC_maincontroller _returnvalue))
  (bind _output (Utilities|Array|Get(acopy) _nearbypickupactors))
  (bind _인벤 (Variables|/Game/RPG/BPC_maincontroller.BPC_maincontroller_C|Get인벤 _asbpc_maincontroller))
  (Networking|SwitchHasAuthority
    (:Authority
      (Development|PrintString "Hello"))
    (:Remote
      (if (== (Pawn|GetController BaiscChar) (Game|GetPlayerController 0))
        (Utilities|IsValid _인벤
          (:Is%20Valid
            (if (== (Variables|Default|GetEnhanceCount) 0)
              (Default|C2SAddItem _인벤 _itemtoadd (Variables|Default|GetAmount))
              (else
                (Default|AddItem(Internal)Enhance _인벤 _itemtoadd 0 0 self)))
            (if (Variables|/Game/InventorySystem/Blueprint/BP_Inventory.BP_Inventory_C|GetAddItemSuccess _인벤)
              (if (> (Variables|/Game/InventorySystem/Blueprint/BP_Inventory.BP_Inventory_C|GetAddItemRest _인벤) 0)
                (Variables|Default|SetAmount 0)
                (CallFunction|UpdateText)
                (else
                  (Utilities|Array|RemoveItem _nearbypickupactors self)
                  (Utilities|IsValid _output
                    (:Is%20Valid
                      (Rendering|SetVisibility (Variables|BP_PickUpActor_C|GetPickupText _output) true false))
                    (:Is%20Not%20Valid
                      _))
                  (if (Variables|Default|GetHovered?)
                    (Variables|/Script/Engine.PlayerController|SetCurrentMouseCursor (Game|GetPlayerController 0) "Default")
                    (Default|C2SDestroyActor BaiscChar self)
                    (else
                      (Default|C2SDestroyActor BaiscChar self))))))))))))

(event Custom|S2A_BeginSetStaticMesh
  (params (NewParam :type Static%20Mesh%20Object%20Reference))
  (Components|StaticMesh|SetStaticMesh (Variables|Default|GetStaticMesh) NewParam))

(event Custom|C2S_BeginSetStaticMesh
  (params (NewParam :type Static%20Mesh%20Object%20Reference))
  (CallFunction|S2ABeginSetStaticMesh NewParam))

(event Custom|C2S_SetEnhanceCount
  (params (Count :type Integer))
  (Variables|Default|SetEnhanceCount Count))

(event EventBeginPlay
  (CallFunction|UpdateText)
  (CallFunction|C2SSetEnhanceCount (Variables|Default|GetEnhanceCount)))

(event Collision|EventActorBeginOverlap
  (params (OtherActor :type Actor%20Object%20Reference)))

(event EventTick
  (params (DeltaSeconds :type Float%20%28single-precision%29)))

(fn ConstructionScript
  (bind _itemtoadd (Variables|Default|GetItemToAdd))
  (bind _staticmesh (Variables|Default|GetStaticMesh))
  (bind _iteminfo (Utilities|GetClassDefaults _itemtoadd))
  (bind (_name _description _icon _canbeused_ _usetext _canbestacked_ _category _weight _value _pickupmesh _meshscale _interactradius) (Utilities|Struct|BreakS_ItemInfo _iteminfo))
  (if (Utilities|IsValidClass _itemtoadd)
    (CallFunction|C2SBeginSetStaticMesh _pickupmesh)
    (Variables|Default|SetOriginalMaterial (Rendering|Material|GetMaterial _staticmesh 0))
    (Transformation|SetRelativeScale3D _staticmesh _meshscale)
    (Components|Sphere|SetSphereRadius (Variables|Default|GetSphere) _interactradius false)))

(fn UpdateText
  (bind _aspickup_text (Utilities|Casting|CastToPickupText (UserInterface|GetUserWidgetObject (Variables|Default|GetPickupText)))
    (:then
      (Rendering|Components|TextRender|SetText (Variables|/Game/InventorySystem/Widget/PickupText.PickupText_C|GetNameText _aspickup_text) (Utilities|Text|FormatText "{Name}  ({Amount})" (.Name (Utilities|Struct|BreakS_ItemInfo (.ItemInfo (Utilities|GetClassDefaults (Variables|Default|GetItemToAdd))))) (Variables|Default|GetAmount))))
    (:CastFailed
      _))
  (return))

(fn SetHighlight
  (params (Highlight :type Boolean))
  (Rendering|SetRenderCustomDepth (Variables|Default|GetStaticMesh) Highlight))

(fn OnHovered
  (Variables|Default|SetHovered? true)
  (Variables|/Script/Engine.PlayerController|SetCurrentMouseCursor (Game|GetPlayerController 0) "Hand")
  (Rendering|Material|SetMaterial (Variables|Default|GetStaticMesh) 0 "/Game/InventorySystem/Material/HoveredPickupMat.HoveredPickupMat")
  (Rendering|SetVisibility (Variables|Default|GetPickupText) true false)
  (return))

(fn OnUnHovered
  (Variables|Default|SetHovered? false)
  (Variables|/Script/Engine.PlayerController|SetCurrentMouseCursor (Game|GetPlayerController 0) "Default")
  (Rendering|Material|SetMaterial (Variables|Default|GetStaticMesh) 0 (Variables|Default|GetOriginalMaterial))
  (Rendering|SetVisibility (Variables|Default|GetPickupText) (Variables|Default|GetIsInRange?) false)
  (return))