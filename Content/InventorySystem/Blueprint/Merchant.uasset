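; Merchant actor that lets the player open a shop when nearby.
; A sphere overlap registers it as the BasicCharacter's nearby merchant and toggles its floating text.
; OnInteract creates a centered shop widget, refreshes the inventory and stops character movement, guarded by a DoOnce.
; OnShopClosed restores walking, refreshes a visible inventory, removes the widget and resets the DoOnce.
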(event OnComponentBeginOverlap(Sphere)
  (params (OverlappedComponent :type Primitive%20Component%20Object%20Reference) (OtherActor :type Actor%20Object%20Reference) (OtherComp :type Primitive%20Component%20Object%20Reference) (OtherBodyIndex :type Integer) (bFromSweep :type Boolean) (SweepResult :type Hit%20Result%20Structure%20%28by%20ref%29))
  (bind _asbasic_character (Utilities|Casting|CastToBasicCharacter OtherActor))
  (Variables|/Game/RPG/BasicCharacter/BasicCharacter.BasicCharacter_C|SetNearbyMerchant _asbasic_character self)
  (Rendering|SetVisibility (Variables|Default|GetMerchantText) true false))

(event OnComponentEndOverlap(Sphere)
  (params (OverlappedComponent :type Primitive%20Component%20Object%20Reference) (OtherActor :type Actor%20Object%20Reference) (OtherComp :type Primitive%20Component%20Object%20Reference) (OtherBodyIndex :type Integer))
  (bind _asbasic_character (Utilities|Casting|CastToBasicCharacter OtherActor))
  (Variables|/Game/RPG/BasicCharacter/BasicCharacter.BasicCharacter_C|SetNearbyMerchant _asbasic_character 0)
  (Rendering|SetVisibility (Variables|Default|GetMerchantText) false false))

(event Custom|OnInteract
  (params (BasicChar :type Basic%20Character%20Object%20Reference))
  (Utilities|FlowControl|DoOnce false
    (:Completed
      (Variables|Default|SetBasicChar BasicChar)
      (bind _returnvalue (UserInterface|CreateWidget "/Game/InventorySystem/Widget/ShopWidget.ShopWidget_C" 0 self (Variables|Default|GetBasicChar)))
      (Variables|Default|SetShopWidget _returnvalue)
      (Class|UserWidget|SetPositioninViewport (Variables|Default|GetShopWidget) "(X=0.000000,Y=0.000000)" true)
      (Class|UserWidget|SetAnchorsinViewport (Variables|Default|GetShopWidget) (Utilities|Struct|MakeAnchors "(X=0.500000,Y=0.500000)" "(X=0.500000,Y=0.500000)"))
      (Class|UserWidget|SetAlignmentinViewport (Variables|Default|GetShopWidget) "(X=0.500000,Y=0.500000)")
      (UserInterface|Viewport|AddtoViewport (Variables|Default|GetShopWidget) 5)
      (Default|HideInventory (Variables|/Game/RPG/BasicCharacter/BasicCharacter.BasicCharacter_C|GetInventoryRef (Variables|Default|GetBasicChar)))
      (Default|ShowInventory (Variables|/Game/RPG/BasicCharacter/BasicCharacter.BasicCharacter_C|GetInventoryRef (Variables|Default|GetBasicChar)))
      (Variables|/Game/RPG/BasicCharacter/BasicCharacter.BasicCharacter_C|SetIsShopOpen? (Variables|Default|GetBasicChar) true)
      (Pawn|Components|CharacterMovement|DisableMovement (Variables|/Script/Engine.Character|GetCharacterMovement (Variables|Default|GetBasicChar)))
      (Components|Movement|StopMovementImmediately (Variables|/Script/Engine.Character|GetCharacterMovement (Variables|Default|GetBasicChar))))))

(event Custom|OnShopClosed
  (Variables|/Game/RPG/BasicCharacter/BasicCharacter.BasicCharacter_C|SetIsShopOpen? (Variables|Default|GetBasicChar) false)
  (Pawn|Components|CharacterMovement|SetMovementMode (Variables|/Script/Engine.Character|GetCharacterMovement (Variables|Default|GetBasicChar)) "MOVE_Walking" 0)
  (if (Variables|/Game/InventorySystem/Blueprint/BP_Inventory.BP_Inventory_C|GetIsVisible? (Variables|/Game/RPG/BasicCharacter/BasicCharacter.BasicCharacter_C|GetInventoryRef (Variables|Default|GetBasicChar)))
    (Default|HideInventory (Variables|/Game/RPG/BasicCharacter/BasicCharacter.BasicCharacter_C|GetInventoryRef (Variables|Default|GetBasicChar)))
    (Default|ShowInventory (Variables|/Game/RPG/BasicCharacter/BasicCharacter.BasicCharacter_C|GetInventoryRef (Variables|Default|GetBasicChar))))
  (Widget|RemovefromParent (Variables|Default|GetShopWidget))
  (Variables|Default|SetShopWidget 0)
  (Utilities|FlowControl|DoOnce false) ; enters at Reset
)

(event EventBeginPlay)

(event Collision|EventActorBeginOverlap
  (params (OtherActor :type Actor%20Object%20Reference)))

(event EventTick
  (params (DeltaSeconds :type Float%20%28single-precision%29)))

(fn ConstructionScript)