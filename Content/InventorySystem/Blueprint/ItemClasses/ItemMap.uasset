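; Map item for the inventory system that shows a world map widget when used.
; OnUsed enables the inventory widget, creates a WorldMap widget with a reference back to this actor, and adds it center-anchored to the main widget's canvas.
; OnRead re-enables the inventory widget, removes the map and destroys the actor.
; Input-mode switching nodes are present but unconnected.
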(event Custom|OnRead
  (Widget|SetIsEnabled (Variables|/Game/InventorySystem/Widget/MainWidget.MainWidget_C|GetInventoryWidget (Variables|/Game/InventorySystem/Blueprint/BP_Inventory.BP_Inventory_C|GetMainWidget (Variables|Default|GetInventory))) true)
  (Widget|RemovefromParent (Variables|Default|GetMapWidget))
  (Actor|DestroyActor))

(event EventBeginPlay
  (|CallParentFunction) ; 지금 이 노드는 비활성 상태입니다. \n핀을 끌어서 다른 노드를 연결하면 활성화됩니다.
)

(event Collision|EventActorBeginOverlap
  (params (OtherActor :type Actor%20Object%20Reference))
  (|CallParentFunction OtherActor) ; 지금 이 노드는 비활성 상태입니다. \n핀을 끌어서 다른 노드를 연결하면 활성화됩니다.
)

(event EventTick
  (params (DeltaSeconds :type Float%20%28single-precision%29))
  (|CallParentFunction DeltaSeconds) ; 지금 이 노드는 비활성 상태입니다. \n핀을 끌어서 다른 노드를 연결하면 활성화됩니다.
)

(event EventEventonUsed
  (Widget|SetIsEnabled (Variables|/Game/InventorySystem/Widget/MainWidget.MainWidget_C|GetInventoryWidget (Variables|/Game/InventorySystem/Blueprint/BP_Inventory.BP_Inventory_C|GetMainWidget (Variables|Default|GetInventory))) true)
  (bind _returnvalue (UserInterface|CreateWidget "/Game/InventorySystem/Widget/WorldMap.WorldMap_C" 0 self))
  (bind _output_get (Variables|Default|SetMapWidget _returnvalue))
  (bind _returnvalue_2 (Class|CanvasPanel|AddChildtoCanvas (Variables|/Game/InventorySystem/Widget/MainWidget.MainWidget_C|GetCanvas (Variables|/Game/InventorySystem/Blueprint/BP_Inventory.BP_Inventory_C|GetMainWidget (Variables|Default|GetInventory))) _output_get))
  (Class|CanvasPanelSlot|SetAnchors _returnvalue_2 (Utilities|Struct|MakeAnchors "(X=0.500000,Y=0.500000)" "(X=0.500000,Y=0.500000)"))
  (Class|CanvasPanelSlot|SetAutoSize _returnvalue_2 true)
  (Class|CanvasPanelSlot|SetPosition _returnvalue_2 "(X=-325.000000,Y=-240.000000)"))

(fn ConstructionScript
  (|CallParentFunction))