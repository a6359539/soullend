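; Player controller for a multiplayer RPG that implements a party system: create, invite, accept or decline, leave, kick and disband.
; Right-click traces a character to select its controller and open a context widget; P toggles the party window.
; Events push updated member lists as parameters to clients for immediate refresh, and invites pass pawns to resolve other players' controllers on the server.
; K opens a TEST listen server.
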(event Custom|파티탈퇴%20사전작업
  ;[1 1 1] 파티탈퇴
  (Utilities|Array|RemoveItem (Variables|Default|Getpartyplayerlist) self)
  (Variables|Default|Setpartymaster 0)
  (for _array_element (Variables|Default|Getpartyplayerlist)
    (bind _output_get (Variables|/Game/RPG/PC_Wonseok.PC_Wonseok_C|Setpartyplayerlist _array_element (Variables|Default|Getpartyplayerlist)))
    (CallFunction|파티탈퇴후처리 _array_element _output_get))
  (Utilities|Array|Clear (Variables|Default|Getpartyplayerlist))
  (CallFunction|파티탈퇴후처리 (Variables|Default|Getpartyplayerlist)))

(event Custom|개별서버%20사전작업
  (params (ip :type Name))
  (Variables|Default|Set아이피주소 ip)
  (CallFunction|CustomEvent0))

(event Custom|setpartylist
  (params (partylist :type Array%20of%20PC%20Wonseok%20Object%20References))
  ;[1 1 1] 파티수락 후 파티초기화  클라에게도 파티정보를 넘겨줌  특징 : 블루프린트에 서버에서 실행은 모든 노드가 끝나야 서버->클라 변수값변경이 이루어짐  이를해결하고 바로 변경된값을 위해선 클라이언트에 tempㄱ값을 받아 직접 적용
  (Variables|Default|Setpartyplayerlist partylist))

(event Custom|파티해체
  (bind _partyplayerlist (Variables|Default|Getpartyplayerlist))
  ;[1 1 1] 파티해체
  (Utilities|Array|Clear _partyplayerlist)
  (bind _output_get (Variables|Default|Setpartymaster 0))
  (CallFunction|파티해체후처리 _partyplayerlist _output_get))

(event Custom|파티탈퇴후처리
  (params (NewParam :type Array%20of%20PC%20Wonseok%20Object%20References))
  ;[1 1 1] 파티탈퇴
  (Variables|Default|Setpartyplayerlist NewParam)
  (if (Utilities|IsValid (Variables|Default|Get파티창))
    (Default|플레이어리스트초기화 (Variables|Default|Get파티창))))

(event Custom|partyafterset
  (params (NewParam :type Sinyoung%20Pratice%20Basic%20Character%201%20Child%20Object%20Reference) (trmp :type Array%20of%20PC%20Wonseok%20Object%20References))
  (bind _파티창 (Variables|Default|Get파티창))
  ;[1 1 1] 파티수락 후 파티초기화  클라에게도 파티정보를 넘겨줌  특징 : 블루프린트에 서버에서 실행은 모든 노드가 끝나야 서버->클라 변수값변경이 이루어짐  이를해결하고 바로 변경된값을 위해선 클라이언트에 tempㄱ값을 받아 직접 적용
  (Variables|Default|Setpartyplayerlist trmp)
  (Utilities|IsValid _파티창
    (:Is%20Valid
      (Default|플레이어리스트초기화 _파티창)
      (if (== NewParam (Game|Player|GetPlayerPawn 0))
        _))))

(event Custom|파티생성
  (bind _partyplayerlist (Variables|Default|Getpartyplayerlist))
  ;[1 1 1] 파티만들기(파티장)
  (if (== (Utilities|Array|Length (Variables|Default|Getpartyplayerlist)) 0)
    (Utilities|Array|Add _partyplayerlist self)
    (bind _output_get (Variables|Default|Setpartymaster self))
    (CallFunction|플레이어리스트초기화 _partyplayerlist _output_get)))

(event Custom|Custom%20Event_0
  (Development|ExecuteConsoleCommand "open TEST?listen"))

(event Custom|파티거절
  ;[1 1 1] 파티거절
  (Variables|/Game/RPG/PC_Wonseok.PC_Wonseok_C|Set파티초대가능? (Variables|Default|Getpartymaster) true)
  (Variables|Default|Setpartymaster 0))

(event Custom|inviteparty
  (params (NewParam :type PC%20Wonseok%20Object%20Reference))
  ;[1 1 1] 파티초대 * 중요정보 다른 클라이언트에게 pc정보를 직접 알려주는게 안되서 파티신청자의 pawn 정보를 넘겨줌     받는 클라는 그 pawn을 이용하여 서버에서 pc를 알아냄
  (Variables|Default|Set파티초대가능? false)
  (Development|PrintString "Hello")
  (if (== (Variables|/Game/RPG/PC_Wonseok.PC_Wonseok_C|Getpartymaster (Variables|Default|Getselectpc)) 0)
    (CallFunction|Masterset (Variables|Default|Getselectpc) (.AsSinyoung%20Pratice%20Basic%20Character%201%20Child (Utilities|Casting|CastTosinyoungPratice_BasicCharacter1_Child (Pawn|GetControlledPawn NewParam))))
    (else
      (Variables|Default|Set파티초대가능? true)
      (CallFunction|이미파티가있는경우))))

(event Custom|파티해체사전작업
  (bind _partyplayerlist (Variables|Default|Getpartyplayerlist))
  ;[1 1 1] 파티해체
  (for (_array_element _array_index) (Variables|Default|Getpartyplayerlist)
    (if (!= _array_index 0)
      (CallFunction|파티해체 _array_element)))
  (Utilities|Array|Clear _partyplayerlist)
  (bind _output_get (Variables|Default|Setpartymaster 0))
  (CallFunction|파티해체후처리 _partyplayerlist _output_get))

(event Custom|set%20selectactor
  (params (NewParam :type Actor%20Object%20Reference))
  ;[1 1 1] 오른쪽클릭 라인트레이스 선택한 캐릭터의 pc selectpcㅇ에 저장
  (if (Variables|Default|Get파티초대가능?)
    (bind _aspc_wonseok (Utilities|Casting|CastToPC_Wonseok (Game|GetInstigatorController NewParam)))
    (Variables|Default|Setselectpc _aspc_wonseok)))

(event Custom|accptserver
  (bind _partyplayerlist (Variables|Default|Getpartyplayerlist))
  ;[1 1 1] 파티수락 후 파티초기화  클라에게도 파티정보를 넘겨줌  특징 : 블루프린트에 서버에서 실행은 모든 노드가 끝나야 서버->클라 변수값변경이 이루어짐  이를해결하고 바로 변경된값을 위해선 클라이언트에 tempㄱ값을 받아 직접 적용
  (Variables|Default|Set파티초대가능? true)
  (Utilities|Array|Add (Variables|Default|Getpartyplayerlist) (Variables|Default|Getselectpc))
  (CallFunction|Setpartylist (Variables|Default|Getselectpc) (Variables|Default|Getpartyplayerlist))
  (for _array_element _partyplayerlist
    (for _array_element_2 _partyplayerlist
      (CallFunction|Partyafterset _array_element (.AsSinyoung%20Pratice%20Basic%20Character%201%20Child (Utilities|Casting|CastTosinyoungPratice_BasicCharacter1_Child (Pawn|GetControlledPawn _array_element_2))) (Variables|Default|Getpartyplayerlist)))))

(event Custom|플레이어리스트%20초기화
  (params (templist :type Array%20of%20PC%20Wonseok%20Object%20References) (tempmaster :type PC%20Wonseok%20Object%20Reference))
  ;[1 1 1] 파티만들기(파티장)
  (Variables|Default|Setpartyplayerlist templist)
  (Variables|Default|Setpartymaster tempmaster)
  (if (Utilities|IsValid (Variables|Default|Get파티창))
    (Default|플레이어리스트초기화 (Variables|Default|Get파티창))))

(event Custom|파티해체%20후처리
  (params (pctemp :type Array%20of%20PC%20Wonseok%20Object%20References) (mastertemp :type PC%20Wonseok%20Object%20Reference))
  (bind _파티창 (Variables|Default|Get파티창))
  ;[1 1 1] 파티해체
  (Variables|Default|Setpartyplayerlist pctemp)
  (Variables|Default|Setpartymaster mastertemp)
  (Utilities|IsValid _파티창
    (:Is%20Valid
      (Default|플레이어리스트초기화 _파티창))))

(event Custom|파티추방%20사전작업
  (params (index :type Integer))
  ;[1 1 1] 파티추방
  (for (_array_element _array_index) (Variables|Default|Getpartyplayerlist)
    (if (== _array_index index)
      (Utilities|Array|Clear (Variables|/Game/RPG/PC_Wonseok.PC_Wonseok_C|Getpartyplayerlist _array_element))
      (Variables|/Game/RPG/PC_Wonseok.PC_Wonseok_C|Setpartymaster _array_element 0)
      (CallFunction|파티추방후처리 _array_element (Variables|/Game/RPG/PC_Wonseok.PC_Wonseok_C|Getpartyplayerlist _array_element))))
  (Utilities|Array|RemoveIndex (Variables|Default|Getpartyplayerlist) index)
  (for _array_element_2 (Variables|Default|Getpartyplayerlist)
    (bind _output_get (Variables|/Game/RPG/PC_Wonseok.PC_Wonseok_C|Setpartyplayerlist _array_element_2 (Variables|Default|Getpartyplayerlist)))
    (CallFunction|파티추방후처리 _array_element_2 _output_get)))

(event Custom|파티추방%20후처리
  (params (templist :type Array%20of%20PC%20Wonseok%20Object%20References))
  ;[1 1 1] 파티추방
  (Variables|Default|Setpartyplayerlist templist)
  (if (Utilities|IsValid (Variables|Default|Get파티창))
    (Default|플레이어리스트초기화 (Variables|Default|Get파티창))))

(event Custom|destroypartywidget
  (Widget|RemovefromParent (Variables|Default|Getpartywidget))
  (Variables|Default|Setpartywidget 0))

(event Custom|이미파티가있는경우
  (bind _returnvalue (UserInterface|CreateWidget "/Game/sinyoung/message.message_C" self))
  (UserInterface|Viewport|AddtoViewport _returnvalue 0))

(event Custom|파티수락
  ;[1 1 1] 상대방이 파티 수락
  (CallFunction|Accptserver (Variables|Default|Getpartymaster)))

(event Custom|partymessagepop
  (params (NewParam :type PC%20Wonseok%20Object%20Reference))
  ;[1 1 1] 위에서 언급했듯이 파티마스터를 저장
  (Variables|Default|Setpartymaster NewParam)
  (bind _returnvalue (UserInterface|CreateWidget "/Game/sinyoung/invitewidget.invitewidget_C" self))
  (UserInterface|Viewport|AddtoViewport _returnvalue 0))

(event Custom|masterset
  (params (masterpc :type Sinyoung%20Pratice%20Basic%20Character%201%20Child%20Object%20Reference))
  ;[1 1 1] 파티초대창 받음
  (bind _output_get (Variables|Default|Setpartymaster (.AsPC%20Wonseok (Utilities|Casting|CastToPC_Wonseok (Pawn|GetController masterpc)))))
  (CallFunction|Partymessagepop _output_get))

(event EventBeginPlay
  (Networking|SwitchHasAuthority
    (:Remote
      (if (== self (Game|GetPlayerController 0))
        (Variables|Default|SetbShowMouseCursor true)))))

(event EventTick
  (params (DeltaSeconds :type Float%20%28single-precision%29)))

(event Input|KeyboardEvents|K
  (params (Key :type Key%20Structure))
  (:Pressed
    (Development|ExecuteConsoleCommand "open TEST?listen")))

(event Input|MouseEvents|RightMouseButton
  (params (Key :type Key%20Structure))
  (bind _returnvalue (Game|GetPlayerController 0))
  (bind _self self)
  (bind (_worldlocation _worlddirection) (Game|Player|ConvertMouseLocationToWorldSpace _returnvalue))
  ;[1 1 1] 오른쪽클릭 라인트레이스 선택한 캐릭터의 pc selectpcㅇ에 저장
  (:Pressed
    (bind (_outhit _returnvalue_2) (Collision|LineTraceForObjects _worldlocation (+ _worldlocation (* _worlddirection 5e+03)) (Utilities|Array|MakeArray "ObjectTypeQuery1" "ObjectTypeQuery3") false 0 "ForOneFrame"))
    (if _returnvalue_2
      (if (!= (.HitActor (Collision|BreakHitResult _outhit)) (Game|Player|GetPlayerPawn 0))
        (Utilities|Casting|CastTosinyoungPratice_BasicCharacter1_Child (.HitActor (Collision|BreakHitResult _outhit)))
        (CallFunction|SetSelectactor (.HitActor (Collision|BreakHitResult _outhit)))
        (if (not (Utilities|IsValid (Variables|Default|Getpartywidget)))
          (bind _returnvalue_3 (UserInterface|CreateWidget "/Game/sinyoung/rightbuttonwidget.rightbuttonwidget_C" _self))
          (Variables|Default|Setpartywidget _returnvalue_3)
          (UserInterface|Viewport|AddtoViewport _returnvalue_3 0)
          (Class|UserWidget|SetPositioninViewport _returnvalue_3 (Math|Vector2D|MakeVector2D (+ (.x (.ScreenPosition (Class|GameplayStatics|ProjectWorldtoScreen _self (.Location (Collision|BreakHitResult _outhit)) false))) 5e+01) (.y (.ScreenPosition (Class|GameplayStatics|ProjectWorldtoScreen _self (.Location (Collision|BreakHitResult _outhit)) false)))) true))))))

(event Input|KeyboardEvents|P
  (params (Key :type Key%20Structure))
  ;[1 1 1] 파티창오픈
  (:Pressed
    (if (Utilities|IsValid (Variables|Default|Get파티창))
      (Widget|RemovefromParent (Variables|Default|Get파티창))
      (Variables|Default|Set파티창 0)
      (else
        (bind _returnvalue (UserInterface|CreateWidget "/Game/sinyoung/partywidget.partywidget_C" self))
        (bind _output_get (Variables|Default|Set파티창 _returnvalue))
        (UserInterface|Viewport|AddtoViewport _output_get 0)))))

(fn ConstructionScript)