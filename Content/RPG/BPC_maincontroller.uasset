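; Main RPG player controller that sets up the UI, character, inventory, party menus and monster targeting.
; Remote BeginPlay creates the HUD and inventory; DB-fed events possess the character and fill level and items, retrying until widget or inventory exists.
; Tab cycles lock-on through an overlap-built monster list; right-click traces players for a party menu.
; Party invite, accept, leave, kick and disband events are empty, their logic disconnected.
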(event Custom|loadinven
  (bind _returnvalue (Game|GetGameInstance))
  (bind _mycharref (Variables|Default|Getmycharref))
  (bind _asmy_bpgame_instance (Utilities|Casting|CastToMyBPGameInstance _returnvalue))
  (bind _inventoryref (Variables|/Game/RPG/BasicCharacter/BasicCharacter.BasicCharacter_C|GetInventoryRef _mycharref))
  (bind _itemtable (Variables|/Script/db.MyGameInstance|Getitemtable _asmy_bpgame_instance))
  (bind (_itemnum _amount _enhance) (Utilities|Struct|BreakMyItemTable _itemtable))
  ;[1 1 1] 인벤셋
  (if (Utilities|IsValid (Variables|Default|Get인벤)) :!label _label
    (for (_array_element _array_index) _itemnum
      (bind _returnvalue_2 (Utilities|GetDataTableRow "/Game/sinyoung/itemtable.itemtable" (Utilities|String|StringToName (Utilities|String|ToString(Integer) _array_element)))
        (:then
          (Utilities|Array|SetArrayElem (Variables|/Game/InventorySystem/Blueprint/BP_Inventory.BP_Inventory_C|GetSlots _inventoryref) _array_index (Utilities|Struct|MakeS_InventorySlot (.itemref _returnvalue_2) (Utilities|Array|Get(acopy) _amount _array_index) (Utilities|Array|Get(acopy) _enhance _array_index) _array_element))
          (Default|UpdateSlotatIndex _inventoryref _array_index))))
    (else
      (Utilities|FlowControl|Delay 0.2)
      (goto _label))))

(event Custom|개별서버%20사전작업
  (params (ip :type Name))
  (Variables|디비변수|Set아이피주소 ip))

(event Custom|2차셋
  (params (NewParam :type Array%20of%20Integers) (NewParam2 :type Array%20of%20Integers) (NewParam3 :type Name))
  ;[1 1 1] DB2차셋
  (Variables|디비변수|Set닉네임 NewParam3)
  (Variables|디비변수|Setuseweaponlv NewParam)
  (Variables|디비변수|Setuseweapoexp NewParam2))

(event Custom|setpartylist
  (params (partylist :type Array%20of%20PC%20Wonseok%20Object%20References))
  ;[1 1 1] 파티
  ;;[1 1 1] 파티수락 후 파티초기화  클라에게도 파티정보를 넘겨줌  특징 : 블루프린트에 서버에서 실행은 모든 노드가 끝나야 서버->클라 변수값변경이 이루어짐  이를해결하고 바로 변경된값을 위해선 클라이언트에 tempㄱ값을 받아 직접 적용
  (Variables|파티|Setpartyplayerlist partylist))

(event Custom|파티해체
  ;[1 1 1] 파티
  ;;[1 1 1] 파티해체
)

(event Custom|파티탈퇴후처리
  (params (NewParam :type Array%20of%20PC%20Wonseok%20Object%20References))
  ;[1 1 1] 파티
  ;;[1 1 1] 파티탈퇴
)

(event Custom|partyafterset
  (params (NewParam :type Sinyoung%20Pratice%20Basic%20Character%201%20Child%20Object%20Reference) (trmp :type Array%20of%20PC%20Wonseok%20Object%20References))
  ;[1 1 1] 파티
  ;;[1 1 1] 파티수락 후 파티초기화  클라에게도 파티정보를 넘겨줌  특징 : 블루프린트에 서버에서 실행은 모든 노드가 끝나야 서버->클라 변수값변경이 이루어짐  이를해결하고 바로 변경된값을 위해선 클라이언트에 tempㄱ값을 받아 직접 적용
)

(event Custom|파티생성
  ;[1 1 1] 파티
  ;;[1 1 1] 파티만들기(파티장)
)

(event Custom|파티거절
  ;[1 1 1] 파티
  ;;[1 1 1] 파티거절
)

(event Custom|inviteparty
  (params (NewParam :type PC%20Wonseok%20Object%20Reference))
  ;[1 1 1] 파티
)

(event Custom|파티해체사전작업
  ;[1 1 1] 파티
  ;;[1 1 1] 파티해체
)

(event Custom|C2S_SetInventoryRef
  (params (Inventory :type BP%20Inventory%20Object%20Reference))
  ;[1 1 1] 메인 ui추가 인벤토리 init
  (Variables|Default|Set인벤 Inventory))

(event Custom|set%20selectactor
  (params (NewParam :type Actor%20Object%20Reference))
  ;[1 1 1] 파티
  ;;[1 1 1] 오른쪽클릭 라인트레이스 선택한 캐릭터의 pc selectpcㅇ에 저장
  (if (Variables|파티|Get파티초대가능?)
    (bind _aspc_wonseok (Utilities|Casting|CastToPC_Wonseok (Game|GetInstigatorController NewParam)))
    (Variables|Default|Setselectpc _aspc_wonseok)))

(event Custom|accptserver
  ;[1 1 1] 파티
  ;;[1 1 1] 파티수락 후 파티초기화  클라에게도 파티정보를 넘겨줌  특징 : 블루프린트에 서버에서 실행은 모든 노드가 끝나야 서버->클라 변수값변경이 이루어짐  이를해결하고 바로 변경된값을 위해선 클라이언트에 tempㄱ값을 받아 직접 적용
)

(event Custom|파티탈퇴%20사전작업
  ;[1 1 1] 파티
  ;;[1 1 1] 파티탈퇴
)

(event Custom|1차셋
  (params (NewParam :type Integer) (NewParam2 :type Integer) (NewParam3 :type Vector))
  ;[1 1 1] DB1차셋
  (bind _returnvalue (Game|SpawnActorfromClass "/Game/RPG/BasicCharacter/realchar.realchar_C" (Math|Transform|MakeTransform NewParam3 "0, 0, 0" "1,1,1") "Undefined" 0 0))
  (bind _output_get (Variables|Default|Setmycharref _returnvalue))
  (Pawn|Possess _returnvalue)
  (bind _output_get_2 (Variables|디비변수|Setlevel NewParam))
  (bind _output_get_3 (Variables|디비변수|Setexp NewParam2))
  (CallFunction|Widget _output_get _output_get_2 _output_get_3)
  (Variables|/Game/InventorySystem/Blueprint/BP_Inventory.BP_Inventory_C|SetBasicCharRef (Variables|Default|Get인벤) (.AsBasic%20Character (Utilities|Casting|CastToBasicCharacter (Game|GetPlayerCharacter 0)))))

(event Custom|플레이어리스트%20초기화
  (params (templist :type Array%20of%20PC%20Wonseok%20Object%20References) (tempmaster :type PC%20Wonseok%20Object%20Reference))
  ;[1 1 1] 파티
  ;;[1 1 1] 파티만들기(파티장)
)

(event Custom|파티해체%20후처리
  (params (pctemp :type Array%20of%20PC%20Wonseok%20Object%20References) (mastertemp :type PC%20Wonseok%20Object%20Reference))
  ;[1 1 1] 파티
  ;;[1 1 1] 파티해체
)

(event Custom|파티추방%20사전작업
  (params (index :type Integer))
  ;[1 1 1] 파티
  ;;[1 1 1] 파티추방
)

(event Custom|파티추방%20후처리
  (params (templist :type Array%20of%20PC%20Wonseok%20Object%20References))
  ;[1 1 1] 파티
  ;;[1 1 1] 파티추방
)

(event Custom|destroypartywidget
  ;[1 1 1] 파티
  (Widget|RemovefromParent (Variables|파티|Getpartywidget))
  (Variables|파티|Setpartywidget 0))

(event Custom|이미파티가있는경우
  ;[1 1 1] 파티
  (bind _returnvalue (UserInterface|CreateWidget "/Game/sinyoung/message.message_C" self))
  (UserInterface|Viewport|AddtoViewport _returnvalue 0))

(event Custom|파티수락
  ;[1 1 1] 파티
  ;;[1 1 1] 상대방이 파티 수락
)

(event Custom|widget
  (params (NewParam :type Realchar%20Object%20Reference) (NewParam2 :type Integer) (NewParam3 :type Integer))
  (bind _mainwidget (Variables|Default|Getmainwidget))
  ;[1 1 1] DB1차위젯셋
  (Variables|Default|Setmycharref NewParam)
  (Variables|디비변수|Setlevel NewParam2)
  (Variables|디비변수|Setexp NewParam3)
  (if (Utilities|IsValid _mainwidget) :!label _label
    (Rendering|Components|TextRender|SetText (Variables|/Game/sinyoung/realwidget.realwidget_C|Getleveltext _mainwidget) (Utilities|Text|FormatText "Lv {t}" (Variables|디비변수|Getlevel)))
    (Progress|SetPercent (Variables|/Game/sinyoung/realwidget.realwidget_C|Getmainlevelexp _mainwidget) (* (/ 1e+04 (Math|Conversions|ToFloat(Integer) (Variables|디비변수|Getexp))) 0.01))
    (else
      (Utilities|FlowControl|Delay 0.2)
      (goto _label))))

(event Custom|partymessagepop
  (params (NewParam :type PC%20Wonseok%20Object%20Reference))
  ;[1 1 1] 파티
  ;;[1 1 1] 위에서 언급했듯이 파티마스터를 저장
)

(event Custom|masterset
  (params (masterpc :type Sinyoung%20Pratice%20Basic%20Character%201%20Child%20Object%20Reference))
  ;[1 1 1] 파티
  ;;[1 1 1] 파티초대창 받음
)

(event EventBeginPlay
  (bind _returnvalue (Game|GetPlayerCharacter 0))
  (bind _asbasic_character (Utilities|Casting|CastToBasicCharacter _returnvalue))
  ;[1 1 1] 메인 ui추가 인벤토리 init
  (Networking|SwitchHasAuthority
    (:Remote
      (bind _asmy_bpgame_instance (Utilities|Casting|CastToMyBPGameInstance (Game|GetGameInstance)))
      (Default|메인서버첫셋팅 _asmy_bpgame_instance)
      (if (== (Game|GetPlayerController 0) self)
        (bind _returnvalue_2 (UserInterface|CreateWidget "/Game/sinyoung/realwidget.realwidget_C" self))
        (Variables|Default|Setmainwidget _returnvalue_2)
        (UserInterface|Viewport|AddtoViewport _returnvalue_2 0)
        (Variables|Default|SetbShowMouseCursor true)
        (Input|SetInputModeGameandUI self 0 "DoNotLock" true)
        (Development|PrintString (Utilities|GetDisplayName _asbasic_character))
        (bind _returnvalue_3 (Game|SpawnActorfromClass "/Game/InventorySystem/Blueprint/BP_Inventory.BP_Inventory_C" (Math|Transform|MakeTransform "0, 0, 0" "0, 0, 0" "1,1,1") "Undefined" 0 20 _asbasic_character 4 1.0 true true 0 0))
        (bind _output_get (Variables|Default|Set인벤 _returnvalue_3))
        (CallFunction|C2SSetInventoryRef _output_get)
        (Default|Init _output_get)))))

(event Input|KeyboardEvents|Tab
  (params (Key :type Key%20Structure))
  (bind _tabmonster (Variables|Default|GetTabMonster))
  (bind _tabmonster_2 (Variables|Default|GetTabMonster))
  (bind _output (Utilities|Array|Get(acopy) _tabmonster_2))
  (bind _output_2 (Utilities|Array|Get(acopy) _tabmonster))
  ;[1 1 1] 자동사냥 베이스가 될 Tab
  (:Pressed
    (bind _asbasic_character (Utilities|Casting|CastToBasicCharacter (Pawn|GetControlledPawn)))
    (Utilities|IsValid _output_2
      (:Is%20Valid
        (Utilities|IsValid (Variables|/Game/RPG/BasicCharacter/BasicCharacter.BasicCharacter_C|GetSelected_Monster _asbasic_character)
          (:Is%20Valid
            (Variables|Default|SetShortMonster _output_2)
            (Development|SetHiddeninGame (Variables|/Game/RPG/Monster/RPG_Monster.RPG_Monster_C|GetParticleSystem (Variables|/Game/RPG/BasicCharacter/BasicCharacter.BasicCharacter_C|GetSelected_Monster _asbasic_character)) true false)
            (Variables|/Game/RPG/Monster/RPG_Monster.RPG_Monster_C|SetLockOn (Variables|/Game/RPG/BasicCharacter/BasicCharacter.BasicCharacter_C|GetSelected_Monster _asbasic_character) false)
            (Effects|Components|ParticleSystem|SetColorParameter (Variables|/Game/RPG/Monster/RPG_Monster.RPG_Monster_C|GetParticleSystem (Variables|/Game/RPG/BasicCharacter/BasicCharacter.BasicCharacter_C|GetSelected_Monster _asbasic_character)) "HoverdToSelectColor" "(R=1.000000,G=1.000000,B=1.000000,A=1.000000)")
            (Default|SelectMonstertoServer _asbasic_character (Variables|Default|GetShortMonster))
            (bind _output_get (Variables|/Game/RPG/BasicCharacter/BasicCharacter.BasicCharacter_C|SetSelected_Monster _asbasic_character (Variables|Default|GetShortMonster)))
            (Effects|Components|ParticleSystem|SetColorParameter (Variables|/Game/RPG/Monster/RPG_Monster.RPG_Monster_C|GetParticleSystem _output_get) "HoverdToSelectColor" "(R=1.000000,G=0.043958,B=0.000000,A=1.000000)")
            (Variables|/Game/RPG/Monster/RPG_Monster.RPG_Monster_C|SetLockOn _output_get true)
            (Development|SetHiddeninGame (Variables|/Game/RPG/Monster/RPG_Monster.RPG_Monster_C|GetParticleSystem _output_get) false false)
            (Utilities|Array|RemoveIndex (Variables|Default|GetTabMonster)))
          (:Is%20Not%20Valid
            (bind _output_get_2 (Variables|Default|SetShortMonster _output_2))
            (Default|SelectMonstertoServer _asbasic_character _output_get_2)
            (bind _output_get_3 (Variables|/Game/RPG/BasicCharacter/BasicCharacter.BasicCharacter_C|SetSelected_Monster _asbasic_character _output_get_2))
            (Utilities|IsValid _output_get_3
              (:Is%20Valid
                (Effects|Components|ParticleSystem|SetColorParameter (Variables|/Game/RPG/Monster/RPG_Monster.RPG_Monster_C|GetParticleSystem _output_get_3) "HoverdToSelectColor" "(R=1.000000,G=0.043958,B=0.000000,A=1.000000)")
                (Development|PrintString (Utilities|GetDisplayName (Variables|/Game/RPG/Monster/RPG_Monster.RPG_Monster_C|GetParticleSystem _output_get_3)))
                (Variables|/Game/RPG/Monster/RPG_Monster.RPG_Monster_C|SetLockOn _output_get_3 true)
                (Development|SetHiddeninGame (Variables|/Game/RPG/Monster/RPG_Monster.RPG_Monster_C|GetParticleSystem _output_get_3) false false)
                (Utilities|Array|RemoveIndex (Variables|Default|GetTabMonster)))))))
      (:Is%20Not%20Valid
        (Variables|Default|SetMonsterIndex 0)
        (bind (_outactors _returnvalue) (Collision|SphereOverlapActors (Transformation|GetActorLocation _asbasic_character) 1e+04 (Utilities|Array|MakeArray "ObjectTypeQuery3") 0 (Utilities|Array|MakeArray _asbasic_character)))
        (if _returnvalue
          (for _array_element _outactors
            (bind _asrpg_monster (Utilities|Casting|CastToRPG_Monster _array_element))
            (Utilities|IsValid _asrpg_monster
              (:Is%20Valid
                (Utilities|Array|AddUnique (Variables|Default|GetTabMonster) _asrpg_monster)
                (Math|Integer|IncrementInt (Variables|Default|GetMonsterIndex)
                  (:%20%20
                    (Development|PrintString "3"))))))
          (Utilities|IsValid (Variables|/Game/RPG/BasicCharacter/BasicCharacter.BasicCharacter_C|GetSelected_Monster _asbasic_character)
            (:Is%20Valid
              (Variables|Default|SetShortMonster _output)
              (Development|SetHiddeninGame (Variables|/Game/RPG/Monster/RPG_Monster.RPG_Monster_C|GetParticleSystem (Variables|/Game/RPG/BasicCharacter/BasicCharacter.BasicCharacter_C|GetSelected_Monster _asbasic_character)) true false)
              (Variables|/Game/RPG/Monster/RPG_Monster.RPG_Monster_C|SetLockOn (Variables|/Game/RPG/BasicCharacter/BasicCharacter.BasicCharacter_C|GetSelected_Monster _asbasic_character) false)
              (Effects|Components|ParticleSystem|SetColorParameter (Variables|/Game/RPG/Monster/RPG_Monster.RPG_Monster_C|GetParticleSystem (Variables|/Game/RPG/BasicCharacter/BasicCharacter.BasicCharacter_C|GetSelected_Monster _asbasic_character)) "HoverdToSelectColor" "(R=1.000000,G=1.000000,B=1.000000,A=1.000000)")
              (Default|SelectMonstertoServer _asbasic_character (Variables|Default|GetShortMonster))
              (bind _output_get_4 (Variables|/Game/RPG/BasicCharacter/BasicCharacter.BasicCharacter_C|SetSelected_Monster _asbasic_character (Variables|Default|GetShortMonster)))
              (Effects|Components|ParticleSystem|SetColorParameter (Variables|/Game/RPG/Monster/RPG_Monster.RPG_Monster_C|GetParticleSystem _output_get_4) "HoverdToSelectColor" "(R=1.000000,G=0.043958,B=0.000000,A=1.000000)")
              (Variables|/Game/RPG/Monster/RPG_Monster.RPG_Monster_C|SetLockOn _output_get_4 true)
              (Development|SetHiddeninGame (Variables|/Game/RPG/Monster/RPG_Monster.RPG_Monster_C|GetParticleSystem _output_get_4) false false)
              (Utilities|Array|RemoveIndex (Variables|Default|GetTabMonster)))
            (:Is%20Not%20Valid
              (bind _output_get_5 (Variables|Default|SetShortMonster _output))
              (Default|SelectMonstertoServer _asbasic_character _output_get_5)
              (bind _output_get_6 (Variables|/Game/RPG/BasicCharacter/BasicCharacter.BasicCharacter_C|SetSelected_Monster _asbasic_character _output_get_5))
              (Utilities|IsValid _output_get_6
                (:Is%20Valid
                  (Effects|Components|ParticleSystem|SetColorParameter (Variables|/Game/RPG/Monster/RPG_Monster.RPG_Monster_C|GetParticleSystem _output_get_6) "HoverdToSelectColor" "(R=1.000000,G=0.043958,B=0.000000,A=1.000000)")
                  (Development|PrintString (Utilities|GetDisplayName (Variables|/Game/RPG/Monster/RPG_Monster.RPG_Monster_C|GetParticleSystem _output_get_6)))
                  (Variables|/Game/RPG/Monster/RPG_Monster.RPG_Monster_C|SetLockOn _output_get_6 true)
                  (Development|SetHiddeninGame (Variables|/Game/RPG/Monster/RPG_Monster.RPG_Monster_C|GetParticleSystem _output_get_6) false false)
                  (Utilities|Array|RemoveIndex (Variables|Default|GetTabMonster)))))))))))

(event Input|MouseEvents|RightMouseButton
  (params (Key :type Key%20Structure))
  (bind _returnvalue (Game|GetPlayerController 0))
  (bind _self self)
  (bind (_worldlocation _worlddirection) (Game|Player|ConvertMouseLocationToWorldSpace _returnvalue))
  ;[1 1 1] 파티
  ;;[1 1 1] 오른쪽클릭 라인트레이스 선택한 캐릭터의 pc selectpcㅇ에 저장
  (:Pressed
    (bind (_outhit _returnvalue_2) (Collision|LineTraceForObjects _worldlocation (+ _worldlocation (* _worlddirection 5e+03)) (Utilities|Array|MakeArray "ObjectTypeQuery1" "ObjectTypeQuery3") false 0 "ForOneFrame"))
    (if _returnvalue_2
      (if (!= (.HitActor (Collision|BreakHitResult _outhit)) (Game|Player|GetPlayerPawn 0))
        (Utilities|Casting|CastTosinyoungPratice_BasicCharacter1_Child (.HitActor (Collision|BreakHitResult _outhit)))
        (CallFunction|SetSelectactor (.HitActor (Collision|BreakHitResult _outhit)))
        (if (not (Utilities|IsValid (Variables|파티|Getpartywidget)))
          (bind _returnvalue_3 (UserInterface|CreateWidget "/Game/sinyoung/rightbuttonwidget.rightbuttonwidget_C" _self))
          (Variables|파티|Setpartywidget _returnvalue_3)
          (UserInterface|Viewport|AddtoViewport _returnvalue_3 0)
          (Class|UserWidget|SetPositioninViewport _returnvalue_3 (Math|Vector2D|MakeVector2D (+ (.x (.ScreenPosition (Class|GameplayStatics|ProjectWorldtoScreen _self (.Location (Collision|BreakHitResult _outhit)) false))) 5e+01) (.y (.ScreenPosition (Class|GameplayStatics|ProjectWorldtoScreen _self (.Location (Collision|BreakHitResult _outhit)) false)))) true))))))

(event Input|KeyboardEvents|P
  (params (Key :type Key%20Structure))
  ;[1 1 1] 파티
  ;;[1 1 1] 파티창오픈
  (:Pressed
    (if (Utilities|IsValid (Variables|파티|Get파티창))
      (Widget|RemovefromParent (Variables|파티|Get파티창))
      (Variables|파티|Set파티창 0)
      (else
        (bind _returnvalue (UserInterface|CreateWidget "/Game/sinyoung/partywidget.partywidget_C" self))
        (bind _output_get (Variables|파티|Set파티창 _returnvalue))
        (UserInterface|Viewport|AddtoViewport _output_get 0)))))

(event Input|KeyboardEvents|J
  (params (Key :type Key%20Structure))
  (:Pressed
    (Development|PrintString "db저장시도")
    (bind _asmy_bpgame_instance (Utilities|Casting|CastToMyBPGameInstance (Game|GetGameInstance)))
    (Default|Saveinven _asmy_bpgame_instance)))

(event Input|KeyboardEvents|I
  (params (Key :type Key%20Structure))
  (bind _인벤 (Variables|Default|Get인벤))
  (:Pressed
    (if (Variables|/Game/InventorySystem/Blueprint/BP_Inventory.BP_Inventory_C|GetIsVisible? (Variables|Default|Get인벤))
      (Default|HideInventory _인벤)
      (else
        (Default|ShowInventory _인벤)))))

(fn ConstructionScript)